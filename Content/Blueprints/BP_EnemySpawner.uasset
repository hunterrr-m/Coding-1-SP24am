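; BP_EnemySpawner spawns waves of BP_Enemy actors across the level's spawn points.
; On BeginPlay it gathers all BP_EnemySpawnLocation actors and spawns an enemy at each with an 80% chance.
; A self-calling check loop, spaced by a short Delay, polls for living BP_Enemy actors and starts another wave when none remain, printing debug messages along the way.
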(event `Spawn Enemies`
  (for _array_element (stale `self.ReceiveBeginPlay` _outactors)
    (if (> (`KismetMathLibrary.RandomFloat`) 0.2)
      (`|SpawnActorFromClass` "/Game/Blueprints/BP_Enemy.BP_Enemy_C" (`self.GetTransform` _array_element) "Undefined" "MultiplyWithRoot" null null))))

(event `self.ReceiveBeginPlay`
  (bind _outactors (`GameplayStatics.GetAllActorsOfClass` "/Game/Blueprints/BP_EnemySpawnLocation.BP_EnemySpawnLocation_C"))
  (`KismetSystemLibrary.PrintString` (`KismetStringLibrary.Concat_StrStr` "There are " (`KismetStringLibrary.Conv_IntToString` (`KismetArrayLibrary.Array_Length` _outactors)) " spawners in the level.") true true (struct :`R` 1.0 :`B` 0.073568 :`A` 1.0))
  (`self.Spawn Enemies`)
  (`self.Check Enemy Count`))

(event `Check Enemy Count`
  (bind _outactors (`GameplayStatics.GetAllActorsOfClass` "/Game/Blueprints/BP_Enemy.BP_Enemy_C"))
  (if (not (> (`KismetArrayLibrary.Array_Length` _outactors) 0))
    (`self.Spawn Enemies`)
    (`KismetSystemLibrary.PrintString` "Another Wave of Enemies have spawned!" true true (struct :`R` 0.55 :`B` 0.020113 :`A` 1.0)))
  (`KismetSystemLibrary.Delay` 0.2)
  (`self.Check Enemy Count`))

(fn `UserConstructionScript`)