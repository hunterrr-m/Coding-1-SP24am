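; Locked door that the third-person character opens by spending a key.
; A hit on the Cube with at least one key calls ChangeKeys(-1), decrements TotalKeys, plays a sound and destroys the door, with a debug message.
; A separate BoxCollision overlap prints a "need a key" message when the character has none.
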(event `self.Cube.OnComponentHit`
  (params (HitComponent :type "PrimitiveComponent Object Reference") (OtherActor :type "Actor Object Reference") (OtherComp :type "PrimitiveComponent Object Reference") (NormalImpulse :type "Vector Structure") (Hit :type "HitResult Structure (by ref)"))
  (bind _asbp_third_person_character (cast `/Game/ThirdPerson/Blueprints/BP_ThirdPersonCharacter` OtherActor))
  (bind _totalkeys (`/Game/ThirdPerson/Blueprints/BP_ThirdPersonCharacter.TotalKeys` _asbp_third_person_character))
  (if (> _totalkeys 0)
    (`/Game/ThirdPerson/Blueprints/BP_ThirdPersonCharacter.ChangeKeys` _asbp_third_person_character -1)
    (`/Engine/EditorBlueprintResources/StandardMacros.DecrementInt` _totalkeys
      (:`  `
        (`GameplayStatics.SpawnSoundAtLocation` "/Game/Audio/Door_Kill_Cue.Door_Kill_Cue" (`SceneComponent.K2_GetComponentLocation` (`self.DefaultSceneRoot`)) (struct) 1.0 1.0 0.0 null null)
        (`self.K2_DestroyActor`)
        (`KismetSystemLibrary.PrintString` "Key Removed. Door Opened." true true (struct :`R` 1.0 :`G` 0.010252 :`B` 0.073962 :`A` 1.0))))))

(event `self.Box Collision.OnComponentBeginOverlap`
  (params (OverlappedComponent :type "PrimitiveComponent Object Reference") (OtherActor :type "Actor Object Reference") (OtherComp :type "PrimitiveComponent Object Reference") (OtherBodyIndex :type Integer) (bFromSweep :type Boolean) (SweepResult :type "HitResult Structure (by ref)"))
  (bind _asbp_third_person_character (cast `/Game/ThirdPerson/Blueprints/BP_ThirdPersonCharacter` OtherActor))
  (if (== (`/Game/ThirdPerson/Blueprints/BP_ThirdPersonCharacter.TotalKeys` _asbp_third_person_character) 0)
    (`KismetSystemLibrary.PrintString` "You need a key!" true true (struct :`R` 0.981074 :`G` 1.0 :`B` 0.856084 :`A` 1.0))))

(fn `UserConstructionScript`)