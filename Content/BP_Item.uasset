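; BP_Item is an item with a name, an elemental type and a damage value that prints debug output on BeginPlay.
; Constructor, called from BeginPlay, attempts to replace a default "Item" name through an array shuffle.
; GetDamage doubles damage against the opposite element, found by offsetting the victim's enum by two with modulo wraparound.
; BeginPlay tests it against Air; an older match-based element check remains unconnected.
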(event `self.ReceiveBeginPlay`
  (`self.Constructor`)
  (`KismetSystemLibrary.PrintString` (`KismetStringLibrary.Concat_StrStr` "debug: " (`self.Name`)) true true (struct :`G` 0.66 :`B` 1.0 :`A` 1.0) 20.0)
  (bind _damage (`self.GetDamage` "NewEnumerator3"))
  (`KismetSystemLibrary.PrintString` (`KismetStringLibrary.Concat_StrStr` "Player element:  " (`|GetEnumeratorNameAsString` (`self.ElementalType`)) " | Victim element: Air | Damage = " (`KismetStringLibrary.Conv_IntToString` _damage)) true true (struct :`R` 0.290343 :`G` 0.161007 :`B` 0.504167 :`A` 1.0) 5.0))

(fn `Constructor`
  (bind _array (`|MakeArray` "One" "Two" "Three"))
  (if (`KismetStringLibrary.EqualEqual_StrStr` (`self.Name`) "Item")
    (`KismetArrayLibrary.Array_Shuffle` _array)
    (bind _output_get (set `self.Name` (`|GetArrayItem` _array)))
    (`KismetSystemLibrary.PrintString` (`KismetStringLibrary.Concat_StrStr` "" _output_get) true true (struct :`G` 0.66 :`B` 1.0 :`A` 1.0) 20.0)))

(fn `GetDamage`
  (params (VictimElemType :type "/Game/ElementalType Enum" :default "NewEnumerator1"))
  (returns (Damage :type Integer))
  (locals (ReturnedDamage :type Integer :default 0))
  (set `local.ReturnedDamage` (`self.Damage`))
  (if (== (mod (+ VictimElemType 2) 4) (`KismetMathLibrary.Conv_ByteToInt` (`self.ElementalType`)))
    (set `local.ReturnedDamage` (* (`self.Damage`) 2))
    (return (`local.ReturnedDamage`))))

(fn `UserConstructionScript`)