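; BP_FunctionExploration is a Blueprint exercise on functions, demonstrated through on-screen debug prints at BeginPlay.
; Say prints text in a random color, and CountToNumber calls it per index with gradually longer durations.
; Each entry in Names prints in a color from GetColorByNameLength: black for short, white for long, gray between.
; The gray uses NormalizeFromRange, which multiplies the offset by its range fraction, so results can exceed 1.
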(event `self.ReceiveBeginPlay`
  (`KismetSystemLibrary.PrintString` "Today's topic is functions!" true true (struct :`R` 0.514876 :`G` 0.491667 :`B` 1.0 :`A` 1.0) 10.0)
  (`self.Say` "Small")
  (`self.CountToNumber` 15)
  (for _array_element (`self.Names`)
    (bind _output (`self.GetColorByNameLength` _array_element))
    (`KismetSystemLibrary.PrintString` _array_element true true _output 10.0)))

(event `Say`
  (params (InString :type String) (Duration :type "Float (single-precision)" :default 5.0))
  (`KismetSystemLibrary.PrintString` InString true true (make `LinearColor` (`KismetMathLibrary.RandomFloat`) (`KismetMathLibrary.RandomFloat`) (`KismetMathLibrary.RandomFloat`) 1.0) Duration))

(fn `CountToNumber`
  (params (Number :type Integer :default 10))
  (for _index (range (+ Number 1))
    (`self.Say` (`KismetStringLibrary.Conv_IntToString` _index) (+ 5.0 (* _index 0.1))))
  (return))

(fn `GetColorByNameLength`
  (params (Input :type String))
  (returns (Output :type "LinearColor Structure"))
  (locals (OutputColor :type "LinearColor Structure"))
  (bind _returnvalue (`KismetStringLibrary.Len` Input))
  (bind _returnvalue_2 (`self.NormalizeFromRange` 5.0 10.0 (`KismetMathLibrary.Conv_IntToDouble` _returnvalue)))
  (if (<= _returnvalue 5)
    (set `local.OutputColor` (make `LinearColor` 0.0 0.0 0.0 1.0))
    (elif (>= _returnvalue 10)
      (set `local.OutputColor` (make `LinearColor` 1.0 1.0 1.0 1.0))
      (else
        (set `local.OutputColor` (make `LinearColor` _returnvalue_2 _returnvalue_2 _returnvalue_2 1.0)))))
  (return (`local.OutputColor`)))

(fn `NormalizeFromRange`
  (params (Min :type "Float (double-precision)" :default 5.0) (Max :type "Float (double-precision)" :default 10.0) (Input :type "Float (double-precision)"))
  (returns (ReturnValue :type "Float (double-precision)"))
  (bind _returnvalue (- Input Min))
  (return (* _returnvalue (/ _returnvalue (- Max Min)))))

(fn `UserConstructionScript`)